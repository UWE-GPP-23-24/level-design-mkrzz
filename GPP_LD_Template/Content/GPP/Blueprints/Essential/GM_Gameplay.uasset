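; Gameplay game mode that runs the level countdown, tracks score and game state, and picks where players start.
; The timer starts at the level duration, counts down each unpaused tick, and triggers a state change whenever it drops below zero and is clamped.
; State changes broadcast through OnStateChanged, and timer progress is exposed as a fraction.
; Player start comes from the checkpoint manager's initial checkpoint.
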(event Custom|ChangeState
  (params (CurrentState :type E_GameStates%20Enum :default "NewEnumerator0"))
  ;[0.4491 0.8591 1] Change State
  (bind _output_get (Variables|Default|SetCurrentState CurrentState))
  (Default|CallOnStateChanged _output_get))

(event EventBeginPlay
  ;[0.4491 0.8591 1] Init timer
  (Variables|Timer|SetLevelTimer (Variables|Timer|GetLevelDuration)))

(event EventTick
  (params (DeltaSeconds :type Float%20%28single-precision%29))
  ;[0.4491 0.8591 1] Decrease timer if not paused
  (if (not (Game|IsGamePaused))
    (CallFunction|DecrementTimer DeltaSeconds)))

(fn ConstructionScript)

(fn ChoosePlayerStart
  (params (Player :type Controller%20Object%20Reference))
  (bind _returnvalue (Actor|GetActorOfClass "/Game/GPP/Blueprints/Checkpoint_System/BP_CheckpointManager.BP_CheckpointManager_C"))
  (bind _initialcheckpoint (Default|GetInitialCheckpoint _returnvalue))
  (return _initialcheckpoint))

(fn AddScore
  (params (Value :type Integer))
  (bind _output_get (Variables|Default|SetScore (+ Value (Variables|Default|GetScore))))
  (Development|PrintString (Utilities|String|ToString(Integer) _output_get)))

(fn GetTimerPercentage
  (return (/ (Variables|Timer|GetLevelTimer) (Variables|Timer|GetLevelDuration))))

(fn DecrementTimer
  (params (DeltaTime :type Float%20%28double-precision%29))
  (bind _output_get (Variables|Timer|SetLevelTimer (- (Variables|Timer|GetLevelTimer) DeltaTime)))
  (if (< _output_get 0.0)
    (Variables|Timer|SetLevelTimer 0.0)
    (CallFunction|ChangeState "NewEnumerator2")))